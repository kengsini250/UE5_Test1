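; MainPlayerController_BP is a player controller that adds animated show and hide transitions to the pause menu.
; It extends the parent DisplayPauseMenu and HiddenPauseMenu events, then casts PauseMenu to HUD_PauseMenu to play PauseMenuAnimation.
; Showing plays the animation forward, while hiding plays it in reverse and sets the widget to Hidden after a short fixed delay.
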(event EventBeginPlay)

(event EventTick
  (params (DeltaSeconds :type Float%20%28single-precision%29)))

(event EventDisplayPauseMenu
  (|CallParentFunction)
  (bind _ashud_pause_menu (Utilities|Casting|CastToHUD_PauseMenu (Variables|Default|GetPauseMenu)))
  (UserInterface|Animation|PlayAnimation _ashud_pause_menu (Variables|/Game/HUD/HUD_PauseMenu.HUD_PauseMenu_C|GetPauseMenuAnimation _ashud_pause_menu) 0.0 1 "Forward" 1.0 false))

(event EventHiddenPauseMenu
  (|CallParentFunction)
  (bind _ashud_pause_menu (Utilities|Casting|CastToHUD_PauseMenu (Variables|Default|GetPauseMenu)))
  (UserInterface|Animation|PlayAnimation _ashud_pause_menu (Variables|/Game/HUD/HUD_PauseMenu.HUD_PauseMenu_C|GetPauseMenuAnimation _ashud_pause_menu) 0.0 1 "Reverse" 1.0 false)
  (Utilities|FlowControl|Delay 0.25)
  (Widget|SetVisibility (Variables|Default|GetPauseMenu) "Hidden"))

(fn ConstructionScript)